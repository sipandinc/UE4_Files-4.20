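; Door actor Blueprint that swings open and closed on alternate calls to its Open event.
; The MyBull boolean selects whether the OpenDoor timeline plays or reverses, then a Sequence node flips it for the next call.
; The timeline's track drives the relative yaw of the Arrow component, which acts as the rotating part of the door.
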(event `/Game/DT_Blueprints/Bp_Interface.open`
  ;[1 1 1] open_Door_process
  (`|ExecutionSequence`
    (:`then_0`
      (if (`self.my bull`)
        (bind (_direction _newtrack_0) (`Timeline|Open door` :!label _label)
          (:`Update`
            (`SceneComponent.K2_SetRelativeRotation` (`self.Arrow`) (`KismetMathLibrary.MakeRotator` 0.0 0.0 _newtrack_0) false false)))
        (else
          (goto _label :!via `Reverse`))))
    (:`then_1`
      (if (`self.my bull`)
        (set `self.my bull` false)
        (else
          (set `self.my bull` true))))))

(fn `UserConstructionScript`)